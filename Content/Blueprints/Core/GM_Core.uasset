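; Game mode for what appears to be an endless runner, managing chunk spawning, game speed, scoring and death.
; It preloads chunks from the BP_BaseSpawner transform, chains each new one to the last chunk's anchor and destroys the oldest with its attached actors.
; Looping timers drive acceleration and score; each speed increase broadcasts the change and resets the speed-derived score interval.
; Death pauses the game and shows the end-game widget with the score.
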(event `self.ReceiveBeginPlay`
  (`|ExecutionSequence`
    (:`then_0`
      ;[0.07245 0.15 0.057 0.5] Init preload Chunks
      (bind _returnvalue (`GameplayStatics.GetActorOfClass` "/Game/Blueprints/BP_BaseSpawner.BP_BaseSpawner_C"))
      (`/Engine/EditorBlueprintResources/StandardMacros.IsValid` _returnvalue
        (:`Is Valid`
          (set `self.SpawnTransform` (`self.GetTransform` _returnvalue))
          (for _ (range 1 (+ (`self.PreloadChunkCount`) 1))
            (`self.SpawnChunk`)))
        (:`Is Not Valid`
          (`KismetSystemLibrary.RaiseScriptError` "Missing a BaseSpawner"))))
    (:`then_1`
      ; Setup Timers
      (`KismetSystemLibrary.K2_SetTimerDelegate` (`|CreateDelegate` :!event `AccelerateGame`) (`self.AccelerationDelay`) true)
      (`self.SetScoreTimer`))))

(event `AccelerateGame`
  (bind _output_get (set `self.currentGameSpeed` (+ (`self.currentGameSpeed`) (`self.AccelerationFactor`))))
  (`self.OnGameSpeedChange` _output_get)
  (`KismetSystemLibrary.K2_ClearAndInvalidateTimerHandle` (`self.ScoreTimer`))
  (`self.SetScoreTimer`)
  (`self.IncreaseScore`))

(event `IncreaseScore`
  ; Increase Score
  (bind _result (`/Engine/EditorBlueprintResources/StandardMacros.IncrementInt` (`self.Score`))
    (:`  `
      (message `/Game/Blueprints/Interfaces/BPI_HUD.UpdateScore` (`PlayerController.GetHUD` (`GameplayStatics.GetPlayerController` 0)) _result))))

(event `/Game/Blueprints/Interfaces/BPI_Game.Death`
  (bind _returnvalue (`GameplayStatics.GetPlayerController` 0))
  (`GameplayStatics.SetGamePaused` true)
  (bind _returnvalue_2 (`|CreateWidget` "/Game/UI/WBP_EndGame.WBP_EndGame_C" _returnvalue (`self.Score`)))
  (`UserWidget.AddToViewport` _returnvalue_2 0)
  (`WidgetBlueprintLibrary.SetInputMode_UIOnlyEx` _returnvalue _returnvalue_2)
  (set `PlayerController.bShowMouseCursor` true _returnvalue))

(fn `clearChunks`
  (locals (listOfActors :type "Array of Actor Object Reference"))
  (bind _output (`|GetArrayItem` (`self.LoadedChunks`)))
  (if (> (`KismetArrayLibrary.Array_Length` (`self.LoadedChunks`)) (+ (`self.PreloadChunkCount`) 1))
    (bind _output_get (set `local.listOfActors` (`self.GetAttachedActors` _output true false)))
    (for _array_element _output_get
      (`self.K2_DestroyActor` _array_element))
    (`self.K2_DestroyActor` _output)
    (`KismetArrayLibrary.Array_RemoveItem` (`self.LoadedChunks`) _output)
    (return)))

(fn `GetCurrentPlaySpeed`
  (returns (gameSpeed :type "Float (double-precision)"))
  (return (`self.currentGameSpeed`)))

(fn `getCurrentSpawnTransform`
  (returns (SpawnTransform :type "Transform Structure"))
  (return (`self.SpawnTransform`)))

(fn `SetScoreTimer`
  (bind _returnvalue (`KismetSystemLibrary.K2_SetTimerDelegate` (`|CreateDelegate` :!event `IncreaseScore`) (/ (`self.currentGameSpeed`) 15.0) true))
  (set `self.ScoreTimer` _returnvalue))

(fn `SpawnChunk`
  (returns (GeneratedChunk :type "/Game/Blueprints/BP_Chunk Object Reference"))
  (bind _loadedchunks (`self.LoadedChunks`))
  (bind _returnvalue (`KismetArrayLibrary.Array_Length` _loadedchunks))
  (bind _output (`|GetArrayItem` _loadedchunks (- _returnvalue 1)))
  (`/Engine/EditorBlueprintResources/StandardMacros.IsValid` _output
    (:`Is Valid`
      (bind _anchortransform (`/Game/Blueprints/BP_Chunk.getChunkAnchorTransform` _output)))
    (:`Is Not Valid`
      _))
  (bind (_returnvalue_location _returnvalue_rotation) (`KismetMathLibrary.BreakTransform` (select `bool` (<= _returnvalue 0) :`false` _anchortransform :`true` (`self.SpawnTransform`))))
  (bind _returnvalue_2 (`|SpawnActorFromClass` "/Game/Blueprints/BP_Chunk.BP_Chunk_C" (`KismetMathLibrary.MakeTransform` _returnvalue_location _returnvalue_rotation) "Undefined" "MultiplyWithRoot" null null))
  (`KismetArrayLibrary.Array_AddUnique` (`self.LoadedChunks`) _returnvalue_2)
  (`self.clearChunks`)
  (return _returnvalue_2))

(fn `UserConstructionScript`)