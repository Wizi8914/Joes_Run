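; Blueprint function library that saves and loads the game's scoreboard through the "ScoreBoards" save slot.
; SaveGameData copies ScoreBoard from the GI_Core game instance into a new BP_Scores save object and writes it to the slot.
; GetGameSave creates the save first if none exists, then loads it, copies ScoreBoard back into GI_Core and returns it.
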(fn `GetGameSave`
  (returns (Output_Get :type "Map of String to Integer"))
  (bind _returnvalue (`GameplayStatics.DoesSaveGameExist` "ScoreBoards"))
  (if (not _returnvalue)
    (`self.SaveGameData` null))
  (bind _returnvalue_2 (`GameplayStatics.LoadGameFromSlot` "ScoreBoards"))
  (`/Engine/EditorBlueprintResources/StandardMacros.IsValid` _returnvalue_2
    (:`Is Valid`
      (bind _asbp_scores (cast `/Game/Blueprints/Saves/BP_Scores` _returnvalue_2))
      (bind _asgi_core (cast `/Game/Blueprints/Core/GI_Core` (`GameplayStatics.GetGameInstance` null)))
      (bind _output_get (set `/Game/Blueprints/Core/GI_Core.ScoreBoard` (`/Game/Blueprints/Saves/BP_Scores.ScoreBoard` _asbp_scores) _asgi_core))
      (return _output_get))))

(fn `SaveGameData`
  (bind _returnvalue (`GameplayStatics.CreateSaveGameObject` "/Game/Blueprints/Saves/BP_Scores.BP_Scores_C"))
  (bind _asgi_core (cast `/Game/Blueprints/Core/GI_Core` (`GameplayStatics.GetGameInstance` null)))
  (set `/Game/Blueprints/Saves/BP_Scores.ScoreBoard` (`/Game/Blueprints/Core/GI_Core.ScoreBoard` _asgi_core) _returnvalue)
  (`GameplayStatics.SaveGameToSlot` _returnvalue "ScoreBoards"))