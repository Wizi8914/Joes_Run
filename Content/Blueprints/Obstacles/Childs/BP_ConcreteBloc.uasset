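; BP_ConcreteBloc is a child obstacle Blueprint with left and right concrete blocks that kill the player on contact.
; Shortly after BeginPlay, it randomly picks one side, hides that obstacle and sets its box to ignore all collision, opening that side.
; Player pawn overlap with either box calls DeathMessage on the Game Mode.
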(event `self.ReceiveBeginPlay`
  (bind _returnvalue (select `int` (`self.Random Index`) :`0` (`self.leftObstacle`) :`1` (`self.RightObstacle`)))
  ;[0.05414 0.15 0.04833 0.5] Init Random Bloc
  (set `self.Random Index` (`KismetMathLibrary.RandomInteger` 2))
  (`KismetSystemLibrary.Delay` 0.2)
  (`/Engine/EditorBlueprintResources/StandardMacros.IsValid` _returnvalue
    (:`Is Valid`
      (`PrimitiveComponent.SetCollisionResponseToAllChannels` (select `int` (`self.Random Index`) :`0` (`self.Box`) :`1` (`self.Box1`)) "ECR_Ignore")
      (`SceneComponent.SetVisibility` _returnvalue false true))))

(event `self.Box.OnComponentBeginOverlap`
  (params (OverlappedComponent :type "PrimitiveComponent Object Reference") (OtherActor :type "Actor Object Reference") (OtherComp :type "PrimitiveComponent Object Reference") (OtherBodyIndex :type Integer) (bFromSweep :type Boolean) (SweepResult :type "HitResult Structure (by ref)"))
  ;[0.15 0.1202 0.0299 0.5] Death
  (if (== OtherActor (`GameplayStatics.GetPlayerPawn` 0))
    (message `/Game/Blueprints/Interfaces/BPI_Game.Death` (`GameplayStatics.GetGameMode`) :!label _label)))

(event `self.Box1.OnComponentBeginOverlap`
  (params (OverlappedComponent :type "PrimitiveComponent Object Reference") (OtherActor :type "Actor Object Reference") (OtherComp :type "PrimitiveComponent Object Reference") (OtherBodyIndex :type Integer) (bFromSweep :type Boolean) (SweepResult :type "HitResult Structure (by ref)"))
  ;[0.15 0.1202 0.0299 0.5] Death
  (if (== OtherActor (`GameplayStatics.GetPlayerPawn` 0))
    (goto _label)))

(fn `UserConstructionScript`
  (`parent.UserConstructionScript`))