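; BP_ConcreteMixer is a child obstacle with center, left and right sections, each paired with a collision box.
; Shortly after BeginPlay, it makes one or two random picks, possibly repeated, hiding those sections and ignoring collision on their boxes to open gaps.
; Overlap of any remaining box by the player pawn calls DeathMessage on the game mode.
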(event `self.ReceiveBeginPlay`
  (bind _returnvalue (select `int` (`self.randomIndex`) :`0` (`self.centerObstacle`) :`1` (`self.leftObstacle`) :`2` (`self.RightObstacle`)))
  (`KismetSystemLibrary.Delay` 0.2)
  (for _ (range (+ (`KismetMathLibrary.RandomInteger` 2) 1))
    (set `self.randomIndex` (`KismetMathLibrary.RandomInteger` 3))
    (`/Engine/EditorBlueprintResources/StandardMacros.IsValid` _returnvalue
      (:`Is Valid`
        (`PrimitiveComponent.SetCollisionResponseToAllChannels` (select `int` (`self.randomIndex`) :`0` (`self.Box`) :`1` (`self.Box1`) :`2` (`self.Box2`)) "ECR_Ignore")
        (`SceneComponent.SetVisibility` _returnvalue false true)))))

(event `self.Box2.OnComponentBeginOverlap`
  (params (OverlappedComponent :type "PrimitiveComponent Object Reference") (OtherActor :type "Actor Object Reference") (OtherComp :type "PrimitiveComponent Object Reference") (OtherBodyIndex :type Integer) (bFromSweep :type Boolean) (SweepResult :type "HitResult Structure (by ref)"))
  (if (== OtherActor (`GameplayStatics.GetPlayerPawn` 0))
    (message `/Game/Blueprints/Interfaces/BPI_Game.Death` (`GameplayStatics.GetGameMode`) :!label _label)))

(event `self.Box1.OnComponentBeginOverlap`
  (params (OverlappedComponent :type "PrimitiveComponent Object Reference") (OtherActor :type "Actor Object Reference") (OtherComp :type "PrimitiveComponent Object Reference") (OtherBodyIndex :type Integer) (bFromSweep :type Boolean) (SweepResult :type "HitResult Structure (by ref)"))
  (if (== OtherActor (`GameplayStatics.GetPlayerPawn` 0))
    (goto _label)))

(event `self.Box.OnComponentBeginOverlap`
  (params (OverlappedComponent :type "PrimitiveComponent Object Reference") (OtherActor :type "Actor Object Reference") (OtherComp :type "PrimitiveComponent Object Reference") (OtherBodyIndex :type Integer) (bFromSweep :type Boolean) (SweepResult :type "HitResult Structure (by ref)"))
  (if (== OtherActor (`GameplayStatics.GetPlayerPawn` 0))
    (goto _label)))

(fn `UserConstructionScript`
  (`parent.UserConstructionScript`))