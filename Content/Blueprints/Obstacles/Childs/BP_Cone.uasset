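; BP_Cone is a child obstacle with center, left and right pieces that can kill the player on overlap.
; Shortly after BeginPlay, it makes one or two random picks, possibly repeated, hiding each picked piece and setting its paired collision to ignore all channels.
; Player overlaps on Capsule1, CenterBarrel or Collision share one path that calls the game mode's DeathMessage.
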(event `self.ReceiveBeginPlay`
  (bind _returnvalue (select `int` (`self.Random Index`) :`0` (`self.centerObstacle`) :`1` (`self.leftObstacle`) :`2` (`self.RightObstacle`)))
  ;[0.03171 0.15 0.05784 0.5] Random Position
  (`KismetSystemLibrary.Delay` 0.2)
  (for _ (range (+ (`KismetMathLibrary.RandomInteger` 2) 1))
    (set `self.Random Index` (`KismetMathLibrary.RandomInteger` 3))
    (`/Engine/EditorBlueprintResources/StandardMacros.IsValid` _returnvalue
      (:`Is Valid`
        (`PrimitiveComponent.SetCollisionResponseToAllChannels` (select `int` (`self.Random Index`) :`0` (`self.Capsule1`) :`1` (`self.Capsule`) :`2` (`self.collision`) :!type "PrimitiveComponent Object Reference") "ECR_Ignore")
        (`SceneComponent.SetVisibility` _returnvalue false true)))))

(event `self.Capsule1.OnComponentBeginOverlap`
  (params (OverlappedComponent :type "PrimitiveComponent Object Reference") (OtherActor :type "Actor Object Reference") (OtherComp :type "PrimitiveComponent Object Reference") (OtherBodyIndex :type Integer) (bFromSweep :type Boolean) (SweepResult :type "HitResult Structure (by ref)"))
  ;[0.15 0.1062 0.05611 0.5] Death
  (if (== OtherActor (`GameplayStatics.GetPlayerPawn` 0))
    (message `/Game/Blueprints/Interfaces/BPI_Game.Death` (`GameplayStatics.GetGameMode`) :!label _label)))

(event `self.centerBarrel.OnComponentBeginOverlap`
  (params (OverlappedComponent :type "PrimitiveComponent Object Reference") (OtherActor :type "Actor Object Reference") (OtherComp :type "PrimitiveComponent Object Reference") (OtherBodyIndex :type Integer) (bFromSweep :type Boolean) (SweepResult :type "HitResult Structure (by ref)"))
  ;[0.15 0.1062 0.05611 0.5] Death
  (if (== OtherActor (`GameplayStatics.GetPlayerPawn` 0))
    (goto _label)))

(event `self.collision.OnComponentBeginOverlap`
  (params (OverlappedComponent :type "PrimitiveComponent Object Reference") (OtherActor :type "Actor Object Reference") (OtherComp :type "PrimitiveComponent Object Reference") (OtherBodyIndex :type Integer) (bFromSweep :type Boolean) (SweepResult :type "HitResult Structure (by ref)"))
  ;[0.15 0.1062 0.05611 0.5] Death
  (if (== OtherActor (`GameplayStatics.GetPlayerPawn` 0))
    (goto _label)))

(fn `UserConstructionScript`
  (`parent.UserConstructionScript`))