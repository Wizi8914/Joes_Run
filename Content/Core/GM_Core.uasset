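; GM_Core is the core game mode that manages a chain of BP_Chunk level pieces and exposes the current game speed and spawn transform.
; On BeginPlay it preloads chunks starting at the BP_BaseSpawner's transform, raising a script error if none exists.
; SpawnChunk attaches each new chunk at the previous one's anchor transform.
; ClearChunks then destroys the oldest chunk once the list exceeds the preload count plus one, keeping a rolling window.
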(event `self.ReceiveBeginPlay`
  (bind _returnvalue (`GameplayStatics.GetActorOfClass` "/Game/Blueprints/BP_BaseSpawner.BP_BaseSpawner_C"))
  (`/Engine/EditorBlueprintResources/StandardMacros.IsValid` _returnvalue
    (:`Is Valid`
      (set `self.SpawnTransform` (`self.GetTransform` _returnvalue))
      (for _ (range 1 (+ (`self.PreloadChunkCount`) 1))
        (`self.SpawnChunk`)))
    (:`Is Not Valid`
      (`KismetSystemLibrary.RaiseScriptError` "Missing a BaseSpawner"))))

(fn `clearChunks`
  (bind _output (`|GetArrayItem` (`self.LoadedChunks`)))
  (if (> (`KismetArrayLibrary.Array_Length` (`self.LoadedChunks`)) (+ (`self.PreloadChunkCount`) 1))
    (`self.K2_DestroyActor` _output)
    (`KismetArrayLibrary.Array_RemoveItem` (`self.LoadedChunks`) _output)))

(fn `GetCurrentPlaySpeed`
  (returns (gameSpeed :type "Float (double-precision)"))
  (return (`self.currentGameSpeed`)))

(fn `getCurrentSpawnTransform`
  (returns (SpawnTransform :type "Transform Structure"))
  (return (`self.SpawnTransform`)))

(fn `SpawnChunk`
  (returns (GeneratedChunk :type "/Game/Blueprints/BP_Chunk Object Reference"))
  (bind _loadedchunks (`self.LoadedChunks`))
  (bind _returnvalue (`KismetArrayLibrary.Array_Length` _loadedchunks))
  (bind _output (`|GetArrayItem` _loadedchunks (- _returnvalue 1)))
  (`/Engine/EditorBlueprintResources/StandardMacros.IsValid` _output
    (:`Is Valid`
      (bind _anchortransform (`/Game/Blueprints/BP_Chunk.getChunkAnchorTransform` _output)))
    (:`Is Not Valid`
      _))
  (bind (_returnvalue_location _returnvalue_rotation) (`KismetMathLibrary.BreakTransform` (select `bool` (<= _returnvalue 0) :`false` _anchortransform :`true` (`self.SpawnTransform`))))
  (bind _returnvalue_2 (`|SpawnActorFromClass` "/Game/Blueprints/BP_Chunk.BP_Chunk_C" (`KismetMathLibrary.MakeTransform` _returnvalue_location _returnvalue_rotation) "Undefined" "MultiplyWithRoot" null null))
  (`KismetArrayLibrary.Array_AddUnique` (`self.LoadedChunks`) _returnvalue_2)
  (`self.clearChunks`)
  (return _returnvalue_2))

(fn `UserConstructionScript`)